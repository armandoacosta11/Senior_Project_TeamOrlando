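; ItemManager is an item factory that spawns item actors in the world from a name.
; CreateItemFromName searches the ItemNames array for the requested name and uses the matching index to pick a class from the parallel ItemTypes array.
; It spawns that class at the given transform and returns the actor, or returns without spawning when the stored index is -1.
; The event graph and construction script are empty.
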(event EventBeginPlay)

(event EventActorBeginOverlap
  (params (OtherActor :type Actor%20Object%20Reference)))

(event EventTick
  (params (DeltaSeconds :type Float%20%28single-precision%29)))

(fn ConstructionScript)

(fn CreateItemfromName
  (params (ItemName :type String) (transform :type Transform))
  (for (_array_element _array_index) (Variables|Default|GetItemNames)
    (if (Utilities|Enum|Equal(Enum) ItemName _array_element)
      (LocalVariables|SetItemPos _array_index)))
  (if (!= (LocalVariables|GetItemPos) -1)
    (bind _returnvalue (Game|SpawnActorfromClass (Utilities|Array|Get(acopy) (Variables|Default|GetItemTypes) (LocalVariables|GetItemPos)) transform "Undefined" 0 0))
    (return _returnvalue)
    (else
      (return 0))))