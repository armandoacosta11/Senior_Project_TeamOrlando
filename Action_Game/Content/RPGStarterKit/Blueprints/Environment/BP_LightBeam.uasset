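; BP_LightBeam is a placeable environment god ray that fakes a visible light shaft with a mesh and material.
; Its construction script adds the mesh, creates a dynamic material instance (optionally animated) and can copy a chosen light actor's rotation.
; Exposed settings drive the beam's shape, color, brightness, fade distance and spotlight or default mask.
; A random stream feeds the material a per-beam variation value.
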(fn `UserConstructionScript`
  (bind _mid (`self.MID`))
  (bind _godraymesh (`self.GodRayMesh`))
  (bind _returnvalue (`AddComponent|StaticMeshComponent_6`))
  (set `self.GodRayMesh` _returnvalue)
  (if (`self.Animated`)
    (bind _returnvalue_2 (`PrimitiveComponent.CreateDynamicMaterialInstance` _godraymesh 0 "/Game/RPGStarterKit/Materials/M_GodRay_Animated.M_GodRay_Animated"))
    (set `self.MID` _returnvalue_2)
    (else
      (bind _returnvalue_3 (`PrimitiveComponent.CreateDynamicMaterialInstance` _godraymesh 0 null))
      (set `self.MID` _returnvalue_3)))
  (if (`self.Use light for rotation`)
    (`SceneComponent.K2_SetRelativeRotation` (`self.GodRayMesh`) (`self.K2_GetActorRotation` (`self.Light`)) true) ; Rotate light beam to match the direction of the light actor
  )
  (if (`self.SpotLight`)
    (`MaterialInstanceDynamic.SetTextureParameterValue` _mid "Mask" "/Game/RPGStarterKit/Textures/T_GodRay_Mask02.T_GodRay_Mask02")
    (else
      (`MaterialInstanceDynamic.SetTextureParameterValue` _mid "Mask" "/Game/RPGStarterKit/Textures/T_GodRay_Mask01.T_GodRay_Mask01")))
  (`MaterialInstanceDynamic.SetScalarParameterValue` _mid "width" (`self.Width`))
  (`MaterialInstanceDynamic.SetScalarParameterValue` _mid "Length" (`self.Length`))
  (`MaterialInstanceDynamic.SetVectorParameterValue` _mid "color" (`self.Color`))
  (`MaterialInstanceDynamic.SetScalarParameterValue` _mid "Brightness" (`self.Brightness`))
  (`MaterialInstanceDynamic.SetScalarParameterValue` _mid "fadedistance" (`self.Fade distance`))
  (`MaterialInstanceDynamic.SetScalarParameterValue` _mid "random" (`KismetMathLibrary.RandomFloatInRangeFromStream` 0.0 100.0 (`self.RandomTime`))))