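; Fireball projectile that flies along its spawn rotation, playing a firing sound when it appears.
; Overlapping an actor sends a DoDamageMessage interface call with BaseDamage; that overlap or a blocking hit spawns explosion effects and sound, then destroys it.
; Without impact, it toggles its particle effect and destroys itself immediately afterward once a fixed lifetime delay ends.
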(event `self.ReceiveBeginPlay`
  ;[1 1 1] Initial setup of the fireball
  (set `MovementComponent.Velocity` (`KismetMathLibrary.GreaterGreater_VectorRotator` (`self.Velocity`) (`self.K2_GetActorRotation`)) (`self.ProjectileMovement`))
  (`GameplayStatics.PlaySoundAtLocation` "/Game/RPGStarterKit/Sounds/FireWeapon_Fire_Cue.FireWeapon_Fire_Cue" (`self.K2_GetActorLocation`))
  (`KismetSystemLibrary.Delay` 5.0) ; Max. Lifetime
  (`ActorComponent.ToggleActive` (`self.Effect`)) ; Turn off effect to give particles a chance to fade instead of disappearing suddenly when the actor is destroyed
  ;[1 1 1] Finally destroy the fireball
  (`self.K2_DestroyActor` :!label _label))

(event `self.ReceiveActorBeginOverlap`
  (params (OtherActor :type "Actor Object Reference"))
  (bind _returnvalue (`self.K2_GetActorLocation`))
  ;[1 1 1] If the fireball hits something, call the interface fuunction so that the fireball can inflict damage
  (message `/Game/RPGStarterKit/Blueprints/Gameplay/BPI_Projectiles.DoDamage` OtherActor (`self.BaseDamage`))
  ;[1 1 1] Play VFX and SFX
  (`GameplayStatics.SpawnEmitterAtLocation` "/Game/RPGStarterKit/ParticleEffects/P_Explosion_Fireball.P_Explosion_Fireball" _returnvalue :!label _label_2)
  (`GameplayStatics.PlaySoundAtLocation` "/Game/RPGStarterKit/Sounds/FireWeapon_Impact_Cue.FireWeapon_Impact_Cue" _returnvalue)
  (goto _label))

(event `self.ReceiveHit`
  (params (MyComp :type "PrimitiveComponent Object Reference") (Other :type "Actor Object Reference") (OtherComp :type "PrimitiveComponent Object Reference") (bSelfMoved :type Boolean) (HitLocation :type "Object.Vector Structure") (HitNormal :type "Object.Vector Structure") (NormalImpulse :type "Object.Vector Structure") (Hit :type "EngineTypes.HitResult Structure (by ref)"))
  ;[1 1 1] Play VFX and SFX
  (goto _label_2))

(fn `UserConstructionScript`)