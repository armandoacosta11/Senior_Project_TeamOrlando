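; Camera actor for the RPG Starter Kit that glides smoothly to a requested location and rotation.
; SmoothMoveToLocation stores the target transform and raises a move flag.
; While that flag is set, Tick eases the actor toward the target with VInterpTo and RInterpTo at CameraInterpSpeed, without sweep.
; Nothing here clears the flag, so interpolation keeps running after the first call.
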(event `self.ReceiveBeginPlay`)

(event `self.ReceiveActorBeginOverlap`
  (params (OtherActor :type "Actor Object Reference")))

(event `self.ReceiveTick`
  (params (DeltaSeconds :type "Float (single-precision)"))
  (bind _camerainterpspeed (`self.CameraInterpSpeed`))
  ;[1 1 1] Move the camera to the new location/rotation
  (if (`self.ShouldMoveToNewLocation`)
    (`self.K2_SetActorLocationAndRotation` (`KismetMathLibrary.VInterpTo` (`self.K2_GetActorLocation`) (`self.LocationToMoveTo`) (`GameplayStatics.GetWorldDeltaSeconds`) _camerainterpspeed) (`KismetMathLibrary.RInterpTo` (`self.K2_GetActorRotation`) (`self.RotationToRotateTo`) (`GameplayStatics.GetWorldDeltaSeconds`) _camerainterpspeed))))

(fn `SmoothMoveToLocation`
  (params (NewLocation :type "Object.Vector Structure" :default (0.0 0.0 0.0)) (NewRotation :type "Object.Rotator Structure" :default (struct)))
  ;[1 1 1] Set the necessary variables for the smooth move. The actual moving is done in the Tick function.
  (set `self.LocationToMoveTo` NewLocation)
  (set `self.RotationToRotateTo` NewRotation)
  (set `self.ShouldMoveToNewLocation` true))

(fn `UserConstructionScript`)